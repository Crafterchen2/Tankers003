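; Tank upgrade helper functions for combining bullet, turret, body and track selections into final tank stats.
; Math Upgrade Function computes a multiplier as level squared times efficiency, plus one.
; Analyse Upgrades holds nodes applying quadratic scaling to fire rate and bullet damage and speed, with turret multipliers on the bullet stats.
; Its entry is unwired, so that struct is never returned, and body health and track speed go unused.
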(fn `Analyse Upgrades`
  (params (BulletIndex :type Integer) (BulletArr :type "Array of /Game/Structures/BulletStruct Structure") (TurretIndex :type Integer) (TurretArr :type "Array of /Game/Structures/TurretStruct Structure") (BodyIndex :type Integer) (BodyArr :type "Array of /Game/Structures/BodyStruct Structure") (TrackIndex :type Integer) (TrackArr :type "Array of /Game/Structures/TrackStruct Structure"))
  (returns (Tank :type "/Game/Structures/FinalTankStruct Structure"))
  (locals (NewLocalVar_0 :type Boolean)))

(fn `Math Upgrade Function`
  (params (Level :type Integer) (UpgradeEfficiency :type "Float (double-precision)"))
  (returns (Multiplier :type "Float (double-precision)"))
  (return (+ (* (* Level Level) UpgradeEfficiency) (- 1.0 0.0))))